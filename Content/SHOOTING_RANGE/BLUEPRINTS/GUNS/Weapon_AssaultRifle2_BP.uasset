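; Assault rifle weapon Blueprint for the shooting range, handling trigger, reload and iron-sight events.
; Pulling the trigger sets a flag and calls FireWeapon in a short RetriggerableDelay loop for automatic fire until release clears the flag.
; Reload calls ReloadWeapon and plays a 2D rifle reload sound.
; Iron-sight on and off both call the same Aim function.
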(event `/Game/SHOOTING_RANGE/BLUEPRINTS/GUNS/Weapon_BP.PullTriger`
  (set `self.IsTriggerPulled` true)
  (`self.FireWeapon` :!label _label)
  ;[1 1 1] Serial Firing
  (`KismetSystemLibrary.RetriggerableDelay` 0.02)
  (if (`self.IsTriggerPulled`)
    (goto _label)))

(event `/Game/SHOOTING_RANGE/BLUEPRINTS/GUNS/Weapon_BP.ReleaseTrigger`
  (set `self.IsTriggerPulled` false))

(event `/Game/SHOOTING_RANGE/BLUEPRINTS/GUNS/Weapon_BP.Reload`
  (`self.ReloadWeapon`)
  (`GameplayStatics.PlaySound2D` "/Game/SHOOTING_RANGE/MESHES/Weapon/MilitaryWeapDark/Sound/Rifle/Rifle_Reload_Cue.Rifle_Reload_Cue" 1.0 1.0 0.0 null null))

(event `/Game/SHOOTING_RANGE/BLUEPRINTS/GUNS/Weapon_BP.IronSightOn`
  (`self.Aim`))

(event `/Game/SHOOTING_RANGE/BLUEPRINTS/GUNS/Weapon_BP.IronSightOff`
  (`self.Aim`))

(fn `UserConstructionScript`
  (`parent.UserConstructionScript`))