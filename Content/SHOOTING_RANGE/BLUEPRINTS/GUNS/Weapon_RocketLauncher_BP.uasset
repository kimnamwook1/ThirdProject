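; Rocket launcher weapon Blueprint for the shooting range, mapping trigger, reload and iron sight events to weapon functions defined outside this file.
; Pulling the trigger sets IsTriggerPulled and calls FireWeapon, while releasing it only clears the flag.
; Reload calls ReloadWeapon, and both iron sight on and off call the same Aim function without arguments.
; BeginPlay, overlap and Tick are disabled stubs, and the construction script only calls its parent.
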(event `/Game/SHOOTING_RANGE/BLUEPRINTS/GUNS/Weapon_BP.PullTriger`
  (set `self.IsTriggerPulled` true)
  (`self.FireWeapon`))

(event `/Game/SHOOTING_RANGE/BLUEPRINTS/GUNS/Weapon_BP.ReleaseTrigger`
  (set `self.IsTriggerPulled` false))

(event `/Game/SHOOTING_RANGE/BLUEPRINTS/GUNS/Weapon_BP.Reload`
  (`self.ReloadWeapon`))

(event `/Game/SHOOTING_RANGE/BLUEPRINTS/GUNS/Weapon_BP.IronSightOn`
  (`self.Aim`))

(event `/Game/SHOOTING_RANGE/BLUEPRINTS/GUNS/Weapon_BP.IronSightOff`
  (`self.Aim`))

(fn `UserConstructionScript`
  (`parent.UserConstructionScript`))