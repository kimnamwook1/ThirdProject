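; Base weapon actor for the shooting range, handling firing, instant reload and aim-down-sights.
; FireWeapon traces from the camera with random spread, then spawns a bullet or launcher grenade at the barrel toward that point, with shake and muzzle effect.
; Non-launcher hits attach decals chosen by component tag.
; Aim blends view between weapon and parent; Aiming is false while sighted, when Tick syncs the hero camera to control rotation.
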(event `self.ReceiveBeginPlay`
  (bind _asb_base_character (cast `/Game/SHOOTING_RANGE/BLUEPRINTS/B_BaseCharacter` (`GameplayStatics.GetPlayerCharacter` 0)))
  (set `self.HeroReference` _asb_base_character))

(event `self.ReceiveTick`
  (params (DeltaSeconds :type "Float (single-precision)"))
  ;[1 1 1] Camera Controller while Aiming
  (if (not (`self.Aiming`))
    (bind _asb_base_character (cast `/Game/SHOOTING_RANGE/BLUEPRINTS/B_BaseCharacter` (`GameplayStatics.GetPlayerCharacter` 0)))
    (`SceneComponent.K2_SetWorldRotation` (`/Game/SHOOTING_RANGE/BLUEPRINTS/B_BaseCharacter.Camera_FPS` _asb_base_character) (`Controller.GetControlRotation` (`GameplayStatics.GetPlayerController` 0)) false false)))

(fn `Aim`
  (if (`self.Aiming`)
    (`PlayerController.SetViewTargetWithBlend` (`GameplayStatics.GetPlayerController` 0) self 0.3 "VTBlend_Linear" 0.0 false)
    (`CameraComponent.SetFieldOfView` (`self.IronSight`) 45.0)
    (set `self.Aiming` false)
    (else
      (`PlayerController.SetViewTargetWithBlend` (`GameplayStatics.GetPlayerController` 0) (`self.GetParentActor`) 0.3 "VTBlend_Linear" 0.0 false)
      (`CameraComponent.SetFieldOfView` (`self.IronSight`) 90.0)
      (set `self.Aiming` true))))

(fn `FireWeapon`
  (bind _returnvalue (`GameplayStatics.GetPlayerCameraManager` 0))
  (bind _accuracy (`self.Accuracy`))
  (bind _returnvalue_2 (`SceneComponent.K2_GetComponentLocation` (`self.Barrel`)))
  (bind _returnvalue_3 (`self.K2_GetActorLocation` _returnvalue))
  (bind _returnvalue_4 (* _accuracy -1.0))
  ;[1 1 1] Fire Condution
  (if (not (`self.IsReloading`))
    (if (>= (`self.ClipActual`) 1)
      (set `self.ClipActual` (- (`self.ClipActual`) 1))
      ;[1 1 1] Line tracing
      (bind (_outhit _returnvalue_5) (`KismetSystemLibrary.LineTraceSingle` _returnvalue_3 (+ (+ (* (`self.GetActorForwardVector` _returnvalue) (`self.Range`)) _returnvalue_3) (`KismetMathLibrary.MakeVector` (`KismetMathLibrary.RandomFloatInRange` _returnvalue_4 _accuracy) (`KismetMathLibrary.RandomFloatInRange` _returnvalue_4 _accuracy) (`KismetMathLibrary.RandomFloatInRange` _returnvalue_4 _accuracy))) "TraceTypeQuery1" false (`|MakeArray` (`self.HeroReference`) :!type "Actor Object Reference")))
      ;[1 1 1] Firing Effect
      (`GameplayStatics.PlayWorldCameraShake` "/Game/SHOOTING_RANGE/BLUEPRINTS/GUNS/Recoil_BP.Recoil_BP_C" (`SceneComponent.K2_GetComponentLocation` (`self.SkeletalMesh`)) 200.0 500.0)
      (if (`self.IsLauncher`)
        (bind (_bblockinghit _binitialoverlap _time _distance _location _impactpoint _normal _impactnormal _physmat _hitactor _hitcomponent _hitbonename _hititem _elementindex _faceindex _tracestart _traceend) (`GameplayStatics.BreakHitResult` _outhit))
        (bind _returnvalue_6 (`KismetMathLibrary.MakeTransform` _returnvalue_2 (`KismetMathLibrary.FindLookAtRotation` _returnvalue_2 (`KismetMathLibrary.SelectVector` _impactpoint _traceend _returnvalue_5))))
        (`|SpawnActorFromClass` "/Game/SHOOTING_RANGE/BLUEPRINTS/GUNS/Granade_BP.Granade_BP_C" _returnvalue_6 "Undefined" "OverrideRootScale" null null)
        (else
          (`|SpawnActorFromClass` "/Game/SHOOTING_RANGE/BLUEPRINTS/GUNS/Bullet_BP.Bullet_BP_C" _returnvalue_6 "Undefined" "OverrideRootScale" null null)))
      (`GameplayStatics.SpawnEmitterAtLocation` "/Game/SHOOTING_RANGE/FX/P_Explosion1.P_Explosion1" (`SceneComponent.K2_GetComponentLocation` (`self.Barrel`)) (struct) (0.17 0.17 0.17))
      (if (not (`self.IsLauncher`))
        ;[1 1 1] Choose Material
        (`/Engine/EditorBlueprintResources/StandardMacros.IsValid` _hitcomponent
          (:`Is Valid`
            (switch `string` (`KismetStringLibrary.Conv_NameToString` (`|GetArrayItem` (`ActorComponent.ComponentTags` _hitcomponent)))
              (:`Steel`
                (bind _returnvalue_7 (`KismetMathLibrary.Conv_VectorToRotator` _normal))
                ;[1 1 1] Attach Bullet Holes
                (`GameplayStatics.SpawnDecalAttached` "/Game/SHOOTING_RANGE/MATERIALS/STEEL_1_M.STEEL_1_M" (`KismetMathLibrary.Conv_DoubleToVector` (`KismetMathLibrary.RandomFloatInRange` 3.0 8.0)) _hitcomponent "None" _location _returnvalue_7 "KeepWorldPosition"))
              (:`Wood`
                (`GameplayStatics.SpawnDecalAttached` "/Game/SHOOTING_RANGE/MATERIALS/WOOD_1_M.WOOD_1_M" (`KismetMathLibrary.Conv_DoubleToVector` (`KismetMathLibrary.RandomFloatInRange` 3.0 8.0)) _hitcomponent "None" _location _returnvalue_7 "KeepWorldPosition"))
              (:`Wall`
                (`GameplayStatics.SpawnDecalAttached` "/Game/SHOOTING_RANGE/MATERIALS/WALL_1_M.WALL_1_M" (`KismetMathLibrary.Conv_DoubleToVector` (`KismetMathLibrary.RandomFloatInRange` 3.0 8.0)) _hitcomponent "None" _location _returnvalue_7 "KeepWorldPosition")
                ;[1 1 1] Dust Effect
                (`GameplayStatics.SpawnEmitterAtLocation` "/Game/SHOOTING_RANGE/FX/P_Impact_Stone_Medium_01.P_Impact_Stone_Medium_01" _location))
              (:`None`
                (`GameplayStatics.SpawnDecalAttached` "/Game/SHOOTING_RANGE/MATERIALS/STEEL_1_M.STEEL_1_M" (`KismetMathLibrary.Conv_DoubleToVector` (`KismetMathLibrary.RandomFloatInRange` 3.0 8.0)) _hitcomponent "None" _location _returnvalue_7 "KeepWorldPosition"))
              (:`Target`
                (`GameplayStatics.SpawnDecalAttached` "/Game/SHOOTING_RANGE/MATERIALS/RED_POINT_M.RED_POINT_M" (3.0 3.0 3.0) _hitcomponent "None" _location _returnvalue_7 "KeepWorldPosition")))))))))

(fn `ReloadWeapon`
  ;[1 1 1] Condition  Check
  (if (not (`self.IsTriggerPulled`))
    (if (not (`self.IsReloading`))
      (if (not (== (`self.ClipActual`) (`self.ClipCapacity`)))
        (if (> (`self.AmmoActual`) 0)
          (set `self.IsReloading` true)
          ;[1 1 1] Reloading
          (bind _output_get (set `self.Required` (- (`self.ClipCapacity`) (`self.ClipActual`))))
          (if (> (`self.AmmoActual`) _output_get)
            (set `self.ClipActual` (`self.ClipCapacity`))
            (set `self.AmmoActual` (- (`self.AmmoActual`) (`self.Required`)))
            (else
              (set `self.ClipActual` (+ (`self.ClipActual`) (`self.AmmoActual`)))
              (set `self.AmmoActual` 0)))
          (set `self.IsReloading` false)
          (return))))))

(fn `UserConstructionScript`)