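; Shooting range target that slides between two positions along a track when a VR player triggers its button.
; BeginPlay caches button and target transforms; an overlap box opens a gate for AddClose only while a VRPawn is inside.
; IsOpen picks forward or reverse timelines that lerp the button, whose updates restart the target's timeline.
; IsMoving blocks retriggering until the target finishes moving.
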(event `self.ReceiveBeginPlay`
  (bind (_returnvalue_location _returnvalue_rotation _returnvalue_scale) (`KismetMathLibrary.BreakTransform` (`SceneComponent.GetRelativeTransform` (`self.Button`))))
  (bind (_returnvalue_location_2 _returnvalue_rotation_2 _returnvalue_scale_2) (`KismetMathLibrary.BreakTransform` (`SceneComponent.GetRelativeTransform` (`self.Target`))))
  ;[1 1 1] Setting Transforms
  (set `self.OutPositionButton` (`KismetMathLibrary.MakeTransform` _returnvalue_location _returnvalue_rotation _returnvalue_scale))
  (set `self.InPositionButton` (`KismetMathLibrary.MakeTransform` (- _returnvalue_location (0.0 0.0 3.0)) _returnvalue_rotation _returnvalue_scale))
  (set `self.OutPositionTarget` (`KismetMathLibrary.MakeTransform` _returnvalue_location_2 _returnvalue_rotation_2 _returnvalue_scale_2))
  (set `self.InPositionTarget` (`KismetMathLibrary.MakeTransform` (+ _returnvalue_location_2 (-3100.0 0.0 0.0)) _returnvalue_rotation_2 _returnvalue_scale_2))
  (`self.EnableInput` (`GameplayStatics.GetPlayerController` 0)))

(event `AddClose`
  ;[1 1 1] Button Interaction(push button)
  (if (not (`self.IsMoving`))
    (`/Engine/EditorBlueprintResources/StandardMacros.Gate` true :!label _label
      (:`Exit`
        (if (`self.IsOpen`)
          ;[1 1 1] Animation
          (bind (_direction _newtrack_0) (`Timeline|Timeline_0` :!via `PlayFromStart`)
            (:`Update`
              (`SceneComponent.K2_SetRelativeTransform` (`self.Button`) (`KismetMathLibrary.TLerp` (`self.OutPositionButton`) (`self.InPositionButton`) _newtrack_0) false false)
              (set `self.IsMoving` true)
              (bind (_direction_2 _newtrack_0_2) (`Timeline|Timeline_1` :!via `PlayFromStart`)
                (:`Update`
                  (`SceneComponent.K2_SetRelativeTransform` (`self.Target`) (`KismetMathLibrary.TLerp` (`self.OutPositionTarget`) (`self.InPositionTarget`) _newtrack_0_2) false false))
                (:`Finished`
                  (set `self.IsOpen` false)
                  (set `self.IsMoving` false)))))
          (else
            (bind (_direction_3 _newtrack_0_3) (`Timeline|Timeline_4` :!via `ReverseFromEnd`)
              (:`Update`
                (`SceneComponent.K2_SetRelativeTransform` (`self.Button`) (`KismetMathLibrary.TLerp` (`self.OutPositionButton`) (`self.InPositionButton`) _newtrack_0_3) false false)
                (set `self.IsMoving` true)
                (bind (_direction_4 _newtrack_0_4) (`Timeline|Timeline_3` :!via `ReverseFromEnd`)
                  (:`Update`
                    (`SceneComponent.K2_SetRelativeTransform` (`self.Target`) (`KismetMathLibrary.TLerp` (`self.OutPositionTarget`) (`self.InPositionTarget`) _newtrack_0_4) false false))
                  (:`Finished`
                    (set `self.IsOpen` true)
                    (set `self.IsMoving` false)))))))))))

(event `self.Box.OnComponentBeginOverlap`
  (params (OverlappedComponent :type "PrimitiveComponent Object Reference") (OtherActor :type "Actor Object Reference") (OtherComp :type "PrimitiveComponent Object Reference") (OtherBodyIndex :type Integer) (bFromSweep :type Boolean) (SweepResult :type "HitResult Structure (by ref)"))
  ;[1 1 1] Button Interaction(push button)
  (cast `/Game/VRTemplate/Blueprints/VRPawn` OtherActor)
  (goto _label :!via `Open`))

(event `self.Box.OnComponentEndOverlap`
  (params (OverlappedComponent :type "PrimitiveComponent Object Reference") (OtherActor :type "Actor Object Reference") (OtherComp :type "PrimitiveComponent Object Reference") (OtherBodyIndex :type Integer))
  ;[1 1 1] Button Interaction(push button)
  (cast `/Game/VRTemplate/Blueprints/VRPawn` OtherActor)
  (goto _label :!via `Close`))

(fn `UserConstructionScript`)