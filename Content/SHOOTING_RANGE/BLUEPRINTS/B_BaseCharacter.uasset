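; Player character for the shooting range, handling movement, look, weapon input and a HUD widget created on BeginPlay.
; Number keys swap the child-actor weapon on the mesh's GripPoint socket, setting its launcher flag and the pistol or rifle AnimBP.
; Fire, reload and toggled aim are forwarded to the weapon as messages.
; E line-traces from the camera to call AddClose on targets, and NightVision toggles post-process when IsNight.
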(event `Key|E`
  (params (Key :type "Key Structure"))
  (bind _returnvalue (`GameplayStatics.GetPlayerCameraManager` 0))
  (bind _returnvalue_2 (`self.K2_GetActorLocation` _returnvalue))
  ;[1 1 1] Line Trace for Interact
  (:`Pressed`
    (bind _outhit (`KismetSystemLibrary.LineTraceSingle` :`Start` _returnvalue_2 :`End` (+ (* (`self.GetActorForwardVector` _returnvalue) 600) _returnvalue_2) :`TraceChannel` "TraceTypeQuery1" :`DrawDebugType` "ForDuration"))
    (bind _astarget_bp (cast `/Game/SHOOTING_RANGE/BLUEPRINTS/Target_BP` (`.HitActor` (`GameplayStatics.BreakHitResult` _outhit))))
    (`/Game/SHOOTING_RANGE/BLUEPRINTS/Target_BP.AddClose` _astarget_bp)))

(event `self.ReceiveBeginPlay`
  ;[1 1 1] widget Visibility
  (bind _returnvalue (`|CreateWidget` "/Game/SHOOTING_RANGE/BLUEPRINTS/HUD_Player.HUD_Player_C" (`GameplayStatics.GetPlayerController` 0)))
  (bind _output_get (set `self.Reference_HUD` _returnvalue))
  (`UserWidget.AddToViewport` _output_get 0)
  (set `self.WidgetVisible` true)
  (`KismetSystemLibrary.Delay` 10.0)
  (set `self.WidgetVisible` false))

(event `Key|One`
  (params (Key :type "Key Structure"))
  (bind _equippedweapon (`self.EquippedWeapon`))
  ;[1 1 1] Pick Weapon
  (:`Pressed`
    (`ChildActorComponent.SetChildActorClass` _equippedweapon "/Game/SHOOTING_RANGE/BLUEPRINTS/GUNS/Weapon_Pistol1_BP.Weapon_Pistol1_BP_C")
    (bind _asweapon_base_bp (cast `/Game/SHOOTING_RANGE/BLUEPRINTS/GUNS/Weapon_Base_BP` (`ChildActorComponent.ChildActor` _equippedweapon)))
    (set `/Game/SHOOTING_RANGE/BLUEPRINTS/GUNS/Weapon_Base_BP.IsLauncher` false _asweapon_base_bp)
    ;[1 1 1] Set Animation
    (`SkeletalMeshComponent.SetAnimInstanceClass` (`self.SkeletalMesh`) "/Game/SHOOTING_RANGE/EpicContent/FirstPerson/Animations/PistolAnimBP.PistolAnimBP_C")))

(event `InputAction|Reload`
  (params (Key :type "Key Structure"))
  ;[1 1 1] Action Input
  (:`Pressed`
    (message `/Game/SHOOTING_RANGE/BLUEPRINTS/GUNS/Weapon_BP.Reload` (`ChildActorComponent.ChildActor` (`self.EquippedWeapon`)))))

(event `InputAction|Jump`
  (params (Key :type "Key Structure"))
  ;[1 1 1] Controller Input
  (:`Pressed`
    (`self.Jump`)))

(event `Key|Two`
  (params (Key :type "Key Structure"))
  (bind _equippedweapon (`self.EquippedWeapon`))
  ;[1 1 1] Pick Weapon
  (:`Pressed`
    (`ChildActorComponent.SetChildActorClass` _equippedweapon "/Game/SHOOTING_RANGE/BLUEPRINTS/GUNS/Weapon_Pistol2_BP.Weapon_Pistol2_BP_C")
    (bind _asweapon_base_bp (cast `/Game/SHOOTING_RANGE/BLUEPRINTS/GUNS/Weapon_Base_BP` (`ChildActorComponent.ChildActor` _equippedweapon)))
    (set `/Game/SHOOTING_RANGE/BLUEPRINTS/GUNS/Weapon_Base_BP.IsLauncher` false _asweapon_base_bp)
    ;[1 1 1] Set Animation
    (`SkeletalMeshComponent.SetAnimInstanceClass` (`self.SkeletalMesh`) "/Game/SHOOTING_RANGE/EpicContent/FirstPerson/Animations/PistolAnimBP.PistolAnimBP_C")))

(event `InputAxis|MoveForward`
  (params (AxisValue :type "Float (single-precision)"))
  ;[1 1 1] Controller Input
  (`self.AddMovementInput` (`self.GetActorForwardVector`) AxisValue))

(event `InputAction|Fire`
  (params (Key :type "Key Structure"))
  (bind _childactor (`ChildActorComponent.ChildActor` (`self.EquippedWeapon`)))
  ;[1 1 1] Action Input
  (:`Pressed`
    (message `/Game/SHOOTING_RANGE/BLUEPRINTS/GUNS/Weapon_BP.PullTriger` _childactor))
  (:`Released`
    (message `/Game/SHOOTING_RANGE/BLUEPRINTS/GUNS/Weapon_BP.ReleaseTrigger` _childactor)))

(event `Key|Three`
  (params (Key :type "Key Structure"))
  (bind _equippedweapon (`self.EquippedWeapon`))
  ;[1 1 1] Pick Weapon
  (:`Pressed`
    (`ChildActorComponent.SetChildActorClass` _equippedweapon "/Game/SHOOTING_RANGE/BLUEPRINTS/GUNS/Weapon_AssaultRifle1_BP.Weapon_AssaultRifle1_BP_C")
    (bind _asweapon_base_bp (cast `/Game/SHOOTING_RANGE/BLUEPRINTS/GUNS/Weapon_Base_BP` (`ChildActorComponent.ChildActor` _equippedweapon)))
    (set `/Game/SHOOTING_RANGE/BLUEPRINTS/GUNS/Weapon_Base_BP.IsLauncher` false _asweapon_base_bp)
    ;[1 1 1] Set Animation
    (`SkeletalMeshComponent.SetAnimInstanceClass` (`self.SkeletalMesh`) "/Game/SHOOTING_RANGE/EpicContent/FirstPerson/Animations/RiffleAnimBP.RiffleAnimBP_C")))

(event `InputAxis|MoveRight`
  (params (AxisValue :type "Float (single-precision)"))
  ;[1 1 1] Controller Input
  (`self.AddMovementInput` (`self.GetActorRightVector`) AxisValue))

(event `InputAction|Aim`
  (params (Key :type "Key Structure"))
  (bind _childactor (`ChildActorComponent.ChildActor` (`self.EquippedWeapon`)))
  ;[1 1 1] Action Input
  (:`Pressed`
    (`/Engine/EditorBlueprintResources/StandardMacros.FlipFlop`
      (:`A`
        (message `/Game/SHOOTING_RANGE/BLUEPRINTS/GUNS/Weapon_BP.IronSightOn` _childactor))
      (:`B`
        (message `/Game/SHOOTING_RANGE/BLUEPRINTS/GUNS/Weapon_BP.IronSightOff` _childactor)))))

(event `Key|Four`
  (params (Key :type "Key Structure"))
  (bind _equippedweapon (`self.EquippedWeapon`))
  ;[1 1 1] Pick Weapon
  (:`Pressed`
    (`ChildActorComponent.SetChildActorClass` _equippedweapon "/Game/SHOOTING_RANGE/BLUEPRINTS/GUNS/Weapon_AssaultRifle2_BP.Weapon_AssaultRifle2_BP_C")
    (bind _asweapon_base_bp (cast `/Game/SHOOTING_RANGE/BLUEPRINTS/GUNS/Weapon_Base_BP` (`ChildActorComponent.ChildActor` _equippedweapon)))
    (set `/Game/SHOOTING_RANGE/BLUEPRINTS/GUNS/Weapon_Base_BP.IsLauncher` false _asweapon_base_bp)
    ;[1 1 1] Set Animation
    (`SkeletalMeshComponent.SetAnimInstanceClass` (`self.SkeletalMesh`) "/Game/SHOOTING_RANGE/EpicContent/FirstPerson/Animations/RiffleAnimBP.RiffleAnimBP_C")))

(event `InputAxis|LookUp`
  (params (AxisValue :type "Float (single-precision)"))
  ;[1 1 1] Controller Input
  (`self.AddControllerPitchInput` AxisValue))

(event `InputAction|NightVision`
  (params (Key :type "Key Structure"))
  (bind _postprocess (`self.PostProcess`))
  ;[1 1 1] Action Input
  (:`Pressed`
    (if (`self.IsNight`)
      (bind _isa (`/Engine/EditorBlueprintResources/StandardMacros.FlipFlop`)
        (:`A`
          (set `PostProcessComponent.bEnabled` _isa _postprocess))
        (:`B`
          (set `PostProcessComponent.bEnabled` _isa _postprocess))))))

(event `Key|Five`
  (params (Key :type "Key Structure"))
  (bind _equippedweapon (`self.EquippedWeapon`))
  ;[1 1 1] Pick Weapon
  (:`Pressed`
    (`ChildActorComponent.SetChildActorClass` _equippedweapon "/Game/SHOOTING_RANGE/BLUEPRINTS/GUNS/Weapon_GranadeLauncher_BP.Weapon_GranadeLauncher_BP_C")
    (bind _asweapon_base_bp (cast `/Game/SHOOTING_RANGE/BLUEPRINTS/GUNS/Weapon_Base_BP` (`ChildActorComponent.ChildActor` _equippedweapon)))
    (set `/Game/SHOOTING_RANGE/BLUEPRINTS/GUNS/Weapon_Base_BP.IsLauncher` true _asweapon_base_bp)
    ;[1 1 1] Set Animation
    (`SkeletalMeshComponent.SetAnimInstanceClass` (`self.SkeletalMesh`) "/Game/SHOOTING_RANGE/EpicContent/FirstPerson/Animations/RiffleAnimBP.RiffleAnimBP_C")))

(event `InputAxis|LookRight`
  (params (AxisValue :type "Float (single-precision)"))
  ;[1 1 1] Controller Input
  (`self.AddControllerYawInput` AxisValue))

(event `Key|Six`
  (params (Key :type "Key Structure"))
  (bind _equippedweapon (`self.EquippedWeapon`))
  ;[1 1 1] Pick Weapon
  (:`Pressed`
    (`ChildActorComponent.SetChildActorClass` _equippedweapon "/Game/SHOOTING_RANGE/BLUEPRINTS/GUNS/Weapon_RocketLauncher_BP.Weapon_RocketLauncher_BP_C")
    (bind _asweapon_base_bp (cast `/Game/SHOOTING_RANGE/BLUEPRINTS/GUNS/Weapon_Base_BP` (`ChildActorComponent.ChildActor` _equippedweapon)))
    (set `/Game/SHOOTING_RANGE/BLUEPRINTS/GUNS/Weapon_Base_BP.IsLauncher` true _asweapon_base_bp)
    ;[1 1 1] Set Animation
    (`SkeletalMeshComponent.SetAnimInstanceClass` (`self.SkeletalMesh`) "/Game/SHOOTING_RANGE/EpicContent/FirstPerson/Animations/RiffleAnimBP.RiffleAnimBP_C")))

(fn `UserConstructionScript`
  (`SceneComponent.K2_AttachToComponent` (`self.EquippedWeapon`) (`self.SkeletalMesh`) "GripPoint" "KeepRelative" "KeepRelative" "KeepRelative" true))