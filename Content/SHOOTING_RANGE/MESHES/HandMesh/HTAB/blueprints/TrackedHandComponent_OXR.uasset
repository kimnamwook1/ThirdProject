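; Actor component for OpenXR hand tracking that gives a pawn with MotionControllers a spawned TrackedHand_OXR actor.
; On BeginPlay it spawns that actor with the chosen skeleton type, then snaps its RHandOXR to each controller whose MotionSource lacks "left", printing an error if none exist.
; No left hand is attached in live logic, and the skeleton switch is empty.
; Laser toggles, beam length, mesh overrides and per-skeleton attachment are disconnected and never run.
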(event `InitAndSpawnHands`
  (bind _returnvalue (`self.GetOwner`))
  ;[1 1 1] Init and Spawn Hands
  (if (!= (`KismetArrayLibrary.Array_Length` (`Actor.K2_GetComponentsByClass` _returnvalue "/Script/HeadMountedDisplay.MotionControllerComponent")) 0)
    (bind _returnvalue_2 (`|SpawnActorFromClass` "/Game/SHOOTING_RANGE/MESHES/HandMesh/HTAB/blueprints/TrackedHand_OXR.TrackedHand_OXR_C" (`SceneComponent.K2_GetComponentToWorld` (`Actor.RootComponent` _returnvalue)) "Undefined" "OverrideRootScale" _returnvalue (`self.Hand Skeleton Type`) null))
    (set `self.thisTrackedHand` _returnvalue_2)))

(event `self.ReceiveBeginPlay`
  (bind _returnvalue (`Actor.K2_GetComponentsByClass` (`self.GetOwner`) "/Script/HeadMountedDisplay.MotionControllerComponent"))
  (`|ExecutionSequence`
    (:`then_0`
      (`self.InitAndSpawnHands`))
    (:`then_1`
      ;[0.3695 1 0.9202] Spawn Default Hand Mesh of either Oculus or Unreal Skeleton
      (switch `/Game/SHOOTING_RANGE/MESHES/HandMesh/HTAB/meshes/HandSkeleton_Type` (`self.Hand Skeleton Type`)))
    (:`then_2`
      (if (!= (`KismetArrayLibrary.Array_Length` _returnvalue) 0)
        (for _array_element _returnvalue
          (if (not (`KismetStringLibrary.Contains` (`KismetStringLibrary.Conv_NameToString` (`MotionControllerComponent.MotionSource` _array_element)) "left"))
            (`SceneComponent.K2_AttachToComponent` (`/Game/SHOOTING_RANGE/MESHES/HandMesh/HTAB/blueprints/TrackedHand_OXR.RHand_OXR` (`self.thisTrackedHand`)) _array_element "None" "SnapToTarget" "SnapToTarget" "KeepWorld" true)))
        (else
          (`KismetSystemLibrary.PrintString` "Error: No MotionControllers Detected, not a valid Pawn"))))
    (:`then_4`)))