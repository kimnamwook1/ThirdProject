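; Tracked-hands VR actor with pinch-driven laser pointers that can trigger mesh swaps on HandPossessor actors.
; Tick uses thumb-index overlaps to toggle lasers and fire clicks, and fingertip distance to scale and fade beams.
; Pinch axes and left-hand clicks call MeshSwapLaserFired on a HandPossessor overlapping the right laser; left clicks add sound and a color flash.
; Right-click handling, skeleton attachment, material setup and capsule generation are disconnected.
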(event `InputAxisKey|OculusHand_Left_IndexPinchStrength`
  (params (AxisValue :type "Float (single-precision)"))
  ;[1 1 1] Pinch Events
  (if (or (> AxisValue 0.0) (> (stale `InputAxisKey|OculusHand_Right_IndexPinchStrength` AxisValue) 0.0)) :!label _label
    ;[0 1 0.4658] Example Custom Fire Event
    (bind _ashand_possessor (cast `/Game/SHOOTING_RANGE/MESHES/HandMesh/HTAB/demo/HandPossessor` (`|GetArrayItem` (`PrimitiveComponent.GetOverlappingActors` (`self.LaserPointer_R`) "/Game/SHOOTING_RANGE/MESHES/HandMesh/HTAB/demo/HandPossessor.HandPossessor_C")) :!label _label_2))
    (`/Game/SHOOTING_RANGE/MESHES/HandMesh/HTAB/demo/HandPossessor.MeshSwapLaserFired` _ashand_possessor self)
    (`KismetSystemLibrary.Delay` 0.2)))

(event `self.ReceiveBeginPlay`
  ;[1 1 1] show lasers by default for UE4 Hands, due to bone limitations
  (`KismetSystemLibrary.Delay` 1.0)
  (switch `/Game/SHOOTING_RANGE/MESHES/HandMesh/HTAB/meshes/HandSkeleton_Type` (`self.HandSkeletonType`)
    (:`NewEnumerator0`
      (`SceneComponent.SetHiddenInGame` (`self.LaserPointer_R`) false false))))

(event `InputAxisKey|OculusHand_Right_IndexPinchStrength`
  (params (AxisValue :type "Float (single-precision)"))
  ;[1 1 1] Pinch Events
  (goto _label))

(event `FireCustomEvent`
  ;[0 1 0.4658] Example Custom Fire Event
  (goto _label_2))

(event `TrackedRHandClickEvent`
  ;[0 1 0.837] Laser Pointer Clicks
)

(event `TrackedRHandUnclickEvent`
  ;[0 1 0.837] Laser Pointer Clicks
)

(event `TrackedLHandClickEvent`
  (bind _lspline_dyn (`self.LSpline_Dyn`))
  ;[0 1 0.837] Laser Pointer Clicks
  (`GameplayStatics.PlaySound2D` "/Game/SHOOTING_RANGE/MESHES/HandMesh/HTAB/blueprints/LaserPointerAssets/click_sound_01B.click_sound_01B" 1.0 1.0 0.0 null null)
  (`MaterialInstanceDynamic.SetVectorParameterValue` _lspline_dyn "LaserColor" (`self.LaserClickColor`))
  (`KismetSystemLibrary.Delay` 0.2)
  (`MaterialInstanceDynamic.SetVectorParameterValue` _lspline_dyn "LaserColor" (`self.LaserHoverColor`))
  (`self.FireCustomEvent`) ; This is whatever logic you want
)

(event `TrackedLHandUnclickEvent`
  ;[0 1 0.837] Laser Pointer Clicks
)

(event `self.ReceiveTick`
  (params (DeltaSeconds :type "Float (single-precision)"))
  (bind _laserinteraction_l (`self.LaserInteraction_L`))
  (bind _laserpointer_r (`self.LaserPointer_R`))
  (bind _laserpointer_l (`self.LaserPointer_L`))
  (bind _laserinteraction_r (`self.LaserInteraction_R`))
  (bind _returnvalue (`KismetMathLibrary.Vector_Distance` (`SceneComponent.K2_GetComponentLocation` (`self.Index_tip_r_click`)) (`SceneComponent.K2_GetComponentLocation` (`self.thumb_tip_r_click`))))
  (bind _returnvalue_2 (`KismetMathLibrary.Vector_Distance` (`SceneComponent.K2_GetComponentLocation` (`self.Index_tip_l_click`)) (`SceneComponent.K2_GetComponentLocation` (`self.thumb_tip_l_click`))))
  (bind _returnvalue_3 (`KismetMathLibrary.MapRangeClamped` _returnvalue 1.0 5.0 0.005 0.075))
  (bind _returnvalue_4 (`KismetMathLibrary.MapRangeClamped` _returnvalue_2 1.0 5.0 0.005 0.075))
  (`|ExecutionSequence`
    (:`then_0`
      ;[1 1 1] Detect if Laser Should be Active
      (if (`PrimitiveComponent.IsOverlappingComponent` (`self.Index_tip_l`) (`self.thumb_tip_l`))
        (`/Engine/EditorBlueprintResources/StandardMacros.DoOnce` false :!label _label_3
          (:`Completed`
            (set `self.isLLaserActive` true)
            (`SceneComponent.SetHiddenInGame` _laserpointer_l false false)
            (`ActorComponent.Activate` _laserinteraction_l false)
            (goto _label_4 :!via `Reset`)))
        (else
          (`|ExecutionSequence`
            (:`then_0`
              (goto _label_3 :!via `Reset`))
            (:`then_1`
              (`/Engine/EditorBlueprintResources/StandardMacros.DoOnce` false :!label _label_4
                (:`Completed`
                  (set `self.isLLaserActive` false)
                  (`SceneComponent.SetHiddenInGame` _laserpointer_l true false)
                  (`ActorComponent.Deactivate` _laserinteraction_l))))))))
    (:`then_1`
      (if (`PrimitiveComponent.IsOverlappingComponent` (`self.Index_tip_r`) (`self.thumb_tip_r`))
        (`/Engine/EditorBlueprintResources/StandardMacros.DoOnce` false :!label _label_5
          (:`Completed`
            (set `self.isRLaserActive` true)
            (`SceneComponent.SetHiddenInGame` _laserpointer_r false false)
            (`ActorComponent.Activate` _laserinteraction_r false)
            (goto _label_6 :!via `Reset`)))
        (else
          (`|ExecutionSequence`
            (:`then_0`
              (goto _label_5 :!via `Reset`))
            (:`then_1`
              (`/Engine/EditorBlueprintResources/StandardMacros.DoOnce` false :!label _label_6
                (:`Completed`
                  (set `self.isRLaserActive` false)
                  (`SceneComponent.SetHiddenInGame` _laserpointer_r true false)
                  (`ActorComponent.Deactivate` _laserinteraction_r))))))))
    (:`then_2`
      ;[1 1 1] Register Finger Click Events
      (if (`PrimitiveComponent.IsOverlappingComponent` (`self.thumb_tip_r_click`) (`self.Index_tip_r_click`))
        (`/Engine/EditorBlueprintResources/StandardMacros.DoOnce` false :!label _label_7
          (:`Completed`
            (`self.TrackedRHandClickEvent`)
            (goto _label_8 :!via `Reset`)))
        (else
          (`|ExecutionSequence`
            (:`then_0`
              (goto _label_7 :!via `Reset`))
            (:`then_1`
              (`/Engine/EditorBlueprintResources/StandardMacros.DoOnce` false :!label _label_8
                (:`Completed`
                  (`self.TrackedRHandUnclickEvent`))))))))
    (:`then_3`
      (if (`PrimitiveComponent.IsOverlappingComponent` (`self.thumb_tip_l_click`) (`self.Index_tip_l_click`))
        (`/Engine/EditorBlueprintResources/StandardMacros.DoOnce` false :!label _label_9
          (:`Completed`
            (`self.TrackedLHandClickEvent`)
            (goto _label_10 :!via `Reset`)))
        (else
          (`|ExecutionSequence`
            (:`then_0`
              (goto _label_9 :!via `Reset`))
            (:`then_1`
              (`/Engine/EditorBlueprintResources/StandardMacros.DoOnce` false :!label _label_10
                (:`Completed`
                  (`self.TrackedLHandUnclickEvent`))))))))
    (:`then_4`
      ;[1 1 1] Laser Dynamic Parameters
      (if (and (`self.isRLaserActive`) (`self.isRLaserEnabled`))
        (`SceneComponent.SetRelativeScale3D` (`self.LaserPointer_R`) (`KismetMathLibrary.MakeVector` _returnvalue_3 _returnvalue_3 (`KismetMathLibrary.MapRangeClamped` _returnvalue 1.0 5.0 1.0 0.001)))
        (`MaterialInstanceDynamic.SetScalarParameterValue` (`self.RSpline_Dyn`) "Opacity" (`KismetMathLibrary.MapRangeClamped` _returnvalue 1.0 3.0 0.05))))
    (:`then_5`
      (if (and (`self.isLLaserEnabled`) (`self.isLLaserEnabled`))
        (`SceneComponent.SetRelativeScale3D` (`self.LaserPointer_L`) (`KismetMathLibrary.MakeVector` _returnvalue_4 _returnvalue_4 (`KismetMathLibrary.MapRangeClamped` _returnvalue_2 1.0 5.0 1.0 0.001)))
        (`MaterialInstanceDynamic.SetScalarParameterValue` (`self.LSpline_Dyn`) "Opacity" (`KismetMathLibrary.MapRangeClamped` _returnvalue_2 1.0 3.0 0.05))))))

(fn `PositionCapsules`
  (params (BoneNamesArray :type "Array of Name") (CapsuleCollArray :type "Array of CapsuleComponent Object Reference") (OculusHand :type "Object Object Reference")))

(fn `UserConstructionScript`)